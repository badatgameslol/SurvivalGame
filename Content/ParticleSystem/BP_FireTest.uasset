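; BP_FireTest is a test fire actor whose flames are switched on and off by player interaction.
; Both the Interaction component and a BP_SurvivalCharacter entering its Sphere toggle IsFireOn, the latter marked as extra test logic.
; The IsFireOn RepNotify activates or deactivates the NSFireWithGlow effect and switches the interaction prompt between TURN OFF and TURN ON.
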(event OnInteract(Interaction)
  (params (Character :type Survival%20Character%20Object%20Reference))
  (Variables|Default|SetIsFireOn (not (Variables|Default|GetIsFireOn))))

(event OnComponentBeginOverlap(Sphere)
  (params (OverlappedComponent :type Primitive%20Component%20Object%20Reference) (OtherActor :type Actor%20Object%20Reference) (OtherComp :type Primitive%20Component%20Object%20Reference) (OtherBodyIndex :type Integer) (bFromSweep :type Boolean) (SweepResult :type Hit%20Result%20Structure%20%28by%20ref%29))
  ;[1 1 1] extra test logic,  it will need to be done to show the items in the inventory ground list
  (bind _asbp_survival_character (Utilities|Casting|CastToBP_SurvivalCharacter OtherActor))
  (if (== OtherActor _asbp_survival_character)
    (Variables|Default|SetIsFireOn (not (Variables|Default|GetIsFireOn)))))

(event EventBeginPlay)

(event Collision|EventActorBeginOverlap
  (params (OtherActor :type Actor%20Object%20Reference)))

(event EventTick
  (params (DeltaSeconds :type Float%20%28single-precision%29)))

(fn ConstructionScript)

(fn OnRepIsFireon
  (bind _ns_firewithglow (Variables|Default|GetNS_FireWithGlow))
  (bind _isfireon (Variables|Default|GetIsFireOn))
  (if _isfireon
    (Components|Activation|Activate _ns_firewithglow _isfireon)
    (else
      (Components|Activation|Deactivate _ns_firewithglow)))
  (Class|InteractionComponent|SetInteractableActionText (Variables|Default|GetInteraction) (select _isfireon (Utilities|Text|MakeLiteralText "TURN OFF") (Utilities|Text|MakeLiteralText "TURN ON"))))