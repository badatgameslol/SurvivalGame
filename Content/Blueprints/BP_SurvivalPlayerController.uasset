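; Player controller for the survival game that toggles the inventory screen with the TestInventoryOpen input action.
; Opening creates WBP_Inventory, adds it to the viewport, focuses it in Game and UI input mode and shows the cursor.
; Closing removes the widget, clears its reference and restores game-only input, so each open builds a fresh widget.
; An open-state flag tracks visibility, and a UI-only input mode node is left unconnected to any event.
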(event Custom|Event_CloseInventory
  ;[1 1 1] Close Inventory
  (Utilities|IsValid (Variables|Default|GetWBP_InventoryRef)
    (:Is%20Valid
      (Widget|RemovefromParent (Variables|Default|GetWBP_InventoryRef))
      (Variables|Default|SetWBP_InventoryRef 0)
      (Input|SetInputModeGameOnly self)
      (Variables|Default|SetbShowMouseCursor false)
      (Variables|Default|SetIsInventoryOpen_0 false))))

(event Custom|Event_OpenInventory
  ;[1 1 1] Open Inventory
  (Utilities|IsValid (Variables|Default|GetWBP_InventoryRef)
    (:Is%20Valid
      _)
    (:Is%20Not%20Valid
      (bind _returnvalue (UserInterface|CreateWidget "/Game/UserInterface/Widgets/WBP_Inventory.WBP_Inventory_C"))
      (Variables|Default|SetWBP_InventoryRef _returnvalue)))
  (UserInterface|Viewport|AddtoViewport (Variables|Default|GetWBP_InventoryRef) 0)
  (Input|SetInputModeGameandUI self (Variables|Default|GetWBP_InventoryRef) "DoNotLock" true)
  (Variables|Default|SetbShowMouseCursor true)
  (Variables|Default|SetIsInventoryOpen_0 true))

(event EventBeginPlay)

(event Input|ActionEvents|InputActionTestInventoryOpen
  (params (Key :type Key%20Structure :default "None"))
  (:Pressed
    (Utilities|IsValid (Variables|Default|GetWBP_InventoryRef)
      (:Is%20Valid
        (CallFunction|EventCloseInventory))
      (:Is%20Not%20Valid
        (CallFunction|EventOpenInventory)))))

(fn ConstructionScript)