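; BP_PickupBase is a base pickup actor that tells the survival character when it is within pickup range.
; Its SphereCollision overlap events cast the other actor to BP_SurvivalCharacter, then add the pickup to that character's PickupItemsInRange on begin and remove it on end.
; Both events print debug strings, and the pickup itself holds no logic for being collected.
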(event OnComponentBeginOverlap(SphereCollision)
  (params (OverlappedComponent :type Primitive%20Component%20Object%20Reference) (OtherActor :type Actor%20Object%20Reference) (OtherComp :type Primitive%20Component%20Object%20Reference) (OtherBodyIndex :type Integer) (bFromSweep :type Boolean) (SweepResult :type Hit%20Result%20Structure%20%28by%20ref%29))
  (bind _asbp_survival_character (Utilities|Casting|CastToBP_SurvivalCharacter OtherActor))
  (if (== OtherActor _asbp_survival_character)
    (Development|PrintString "Hello")
    (Utilities|Array|Add (Variables|/Game/Blueprints/BP_SurvivalCharacter.BP_SurvivalCharacter_C|GetPickupItemsInRange _asbp_survival_character) self)))

(event OnComponentEndOverlap(SphereCollision)
  (params (OverlappedComponent :type Primitive%20Component%20Object%20Reference) (OtherActor :type Actor%20Object%20Reference) (OtherComp :type Primitive%20Component%20Object%20Reference) (OtherBodyIndex :type Integer))
  (bind _asbp_survival_character (Utilities|Casting|CastToBP_SurvivalCharacter OtherActor))
  (if (== OtherActor _asbp_survival_character)
    (Development|PrintString "bello")
    (Utilities|Array|RemoveItem (Variables|/Game/Blueprints/BP_SurvivalCharacter.BP_SurvivalCharacter_C|GetPickupItemsInRange _asbp_survival_character) self)))

(event EventBeginPlay)

(event Collision|EventActorBeginOverlap
  (params (OtherActor :type Actor%20Object%20Reference)))

(event EventTick
  (params (DeltaSeconds :type Float%20%28single-precision%29)))

(fn ConstructionScript)